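; Player actor for a maze game that handles movement, camera control, element selection and switch toggling.
; Forward input pushes the Cylinder with physics impulses, sideways input yaws the actor, and BeginPlay attaches the root to the Cylinder.
; Tick rotates the SpringArm from input axes.
; Number keys map to Elements indices, moving the in-use flag to the chosen element, and another action toggles the referenced Switch if valid.
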(event `InputAction|UseElement`
  (params (Key :type "Key Structure" :default "AnyKey"))
  (bind _returnvalue (`KismetStringLibrary.Conv_StringToInt` (`KismetTextLibrary.Conv_TextToString` (`KismetInputLibrary.Key_GetDisplayName` Key))))
  (:`Pressed`
    (if (<= _returnvalue (`KismetArrayLibrary.Array_Length` (`self.Elements`)))
      (`self.handleElement` (- _returnvalue 1)))))

(event `InputAction|ToggleSwitch`
  (params (Key :type "Key Structure" :default "AnyKey"))
  (bind _switch (`self.switch`))
  (:`Pressed`
    (`/Engine/EditorBlueprintResources/StandardMacros.IsValid` _switch
      (:`Is Valid`
        (`/Game/MazeRunnerAssets/Blueprints/MapAsset/Switch.toggleSwitch` _switch)))))

(event `InputAxis|ForwardOrBackward`
  (params (AxisValue :type "Float (single-precision)"))
  (`PrimitiveComponent.AddImpulse` (`self.Cylinder`) (* (`self.GetActorForwardVector` self) (* AxisValue (`self.speed`))) "None" false))

(event `InputAxis|LeftOrRight`
  (params (AxisValue :type "Float (single-precision)"))
  (`self.K2_AddActorWorldRotation` (`KismetMathLibrary.MakeRotator` 0.0 0.0 (* AxisValue (`self.turnSpeed`)))))

(event `self.ReceiveBeginPlay`
  (`self.K2_AttachRootComponentTo` (`self.Cylinder`) "None" "KeepWorldPosition"))

(event `self.ReceiveActorBeginOverlap`
  (params (OtherActor :type "Actor Object Reference")))

(event `self.ReceiveTick`
  (params (DeltaSeconds :type "Float (single-precision)"))
  (`SceneComponent.K2_AddRelativeRotation` (`self.SpringArm`) (`KismetMathLibrary.MakeRotator` 0.0 (`self.GetInputAxisKeyValue`) (`self.GetInputAxisKeyValue`)) false false))

(fn `handleElement`
  (params (elementIndex :type Integer))
  (bind _elementinhandle (`self.ElementInHandle`))
  (`/Engine/EditorBlueprintResources/StandardMacros.IsValid` _elementinhandle
    (:`Is Valid`
      (set `/Game/MazeRunnerAssets/Blueprints/Element/Element.isInUse` false _elementinhandle))
    (:`Is Not Valid`
      _))
  (bind _output_get (set `self.ElementInHandle` (`KismetArrayLibrary.Array_Get` (`self.Elements`) elementIndex)))
  (set `/Game/MazeRunnerAssets/Blueprints/Element/Element.isInUse` true _output_get)
  (`KismetSystemLibrary.PrintString` (`KismetStringLibrary.Conv_NameToString` (`|GetEnumeratorName` (`/Game/MazeRunnerAssets/Blueprints/Element/Element.ElementType` _output_get)))))

(fn `UserConstructionScript`)