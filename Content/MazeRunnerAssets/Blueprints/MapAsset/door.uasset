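; Double sliding door for a map, which toggles open or closed whenever an actor begins or ends overlap while it is enabled.
; Tick slides both panels apart by a fixed step per frame up to the open length, or back to their saved start positions, then switches itself off.
; SwitchFunction toggles whether the door responds.
; A helper, unused here, can add a child actor wall at a given transform.
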(event `self.ReceiveBeginPlay`
  (set `self.firstPositionOfLeftDoor` (`SceneComponent.K2_GetComponentLocation` (`self.doorLeft`)))
  (set `self.firstPositionOfRightDoor` (`SceneComponent.K2_GetComponentLocation` (`self.doorRight`))))

(event `self.ReceiveActorBeginOverlap`
  (params (OtherActor :type "Actor Object Reference"))
  (if (`self.enableDoor`) :!label _label
    (set `self.doorOnMove` true)
    (`self.toggleDoor`)))

(event `self.ReceiveActorEndOverlap`
  (params (OtherActor :type "Actor Object Reference"))
  (goto _label))

(event `self.ReceiveTick`
  (params (DeltaSeconds :type "Float (single-precision)"))
  (bind _returnvalue (`KismetMathLibrary.VSize` (- (`SceneComponent.K2_GetComponentLocation` (`self.doorLeft`)) (`self.firstPositionOfLeftDoor`))))
  (if (`self.doorOnMove`)
    (if (`self.doorOpen`)
      (`SceneComponent.K2_AddLocalOffset` (`self.doorLeft`) (-1.0 0.0 0.0) false false)
      (`SceneComponent.K2_AddLocalOffset` (`self.doorRight`) (1.0 0.0 0.0) false false)
      (if (>= _returnvalue (`self.doorOpenLength`))
        (set `self.doorOnMove` false)
        (`self.SetActorTickEnabled` false))
      (else
        (`SceneComponent.K2_AddLocalOffset` (`self.doorLeft`) (1.0 0.0 0.0) false false)
        (`SceneComponent.K2_AddLocalOffset` (`self.doorRight`) (-1.0 0.0 0.0) false false)
        (if (< _returnvalue 1.0)
          (set `self.doorOnMove` false)
          (`SceneComponent.K2_SetWorldLocation` (`self.doorLeft`) (`self.firstPositionOfLeftDoor`) false false)
          (`SceneComponent.K2_SetWorldLocation` (`self.doorRight`) (`self.firstPositionOfRightDoor`) false false)
          (`self.SetActorTickEnabled` false))))))

(event `self.switchFunction`
  (`self.toggleEngbleDoor`))

(fn `MakeWallAtPosition`
  (params (makeOrNot :type Boolean) (position :type "Vector Structure") (rotation :type "Rotator Structure"))
  (if makeOrNot
    (`AddComponent|Child Actor Component_2511` :`RelativeTransform` (`KismetMathLibrary.MakeTransform` position rotation))))

(fn `toggleDoor`
  (if (`self.doorOpen`)
    (set `self.doorOpen` false)
    (else
      (set `self.doorOpen` true)))
  (`self.SetActorTickEnabled` true))

(fn `toggleEngbleDoor`
  (if (`self.enableDoor`)
    (set `self.enableDoor` false)
    (else
      (set `self.enableDoor` true))))

(fn `UserConstructionScript`)