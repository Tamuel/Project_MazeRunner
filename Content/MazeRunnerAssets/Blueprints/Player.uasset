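; Player pawn for a maze runner game that moves by physics, turns, orbits its camera and toggles a referenced Switch.
; Forward input applies impulses to the Cylinder along the actor's forward vector, while sideways input yaws the actor.
; BeginPlay calls AttachRootComponentTo with the Cylinder as parent, keeping world position.
; Tick rotates the SpringArm in pitch and yaw from axis key values.
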(event `InputAction|ToggleSwitch`
  (params (Key :type "Key Structure" :default "AnyKey"))
  (bind _switch (`self.switch`))
  (:`Pressed`
    (`/Engine/EditorBlueprintResources/StandardMacros.IsValid` _switch
      (:`Is Valid`
        (`/Game/MazeRunnerAssets/Blueprints/Switch.toggleSwitch` _switch)))))

(event `InputAxis|ForwardOrBackward`
  (params (AxisValue :type "Float (single-precision)"))
  (`PrimitiveComponent.AddImpulse` (`self.Cylinder`) (* (`self.GetActorForwardVector` self) (* AxisValue (`self.speed`))) "None" false))

(event `InputAxis|LeftOrRight`
  (params (AxisValue :type "Float (single-precision)"))
  (`self.K2_AddActorWorldRotation` (`KismetMathLibrary.MakeRotator` 0.0 0.0 (* AxisValue (`self.turnSpeed`)))))

(event `self.ReceiveBeginPlay`
  (`self.K2_AttachRootComponentTo` (`self.Cylinder`) "None" "KeepWorldPosition"))

(event `self.ReceiveActorBeginOverlap`
  (params (OtherActor :type "Actor Object Reference")))

(event `self.ReceiveTick`
  (params (DeltaSeconds :type "Float (single-precision)"))
  (`SceneComponent.K2_AddRelativeRotation` (`self.SpringArm`) (`KismetMathLibrary.MakeRotator` 0.0 (`self.GetInputAxisKeyValue`) (`self.GetInputAxisKeyValue`)) false false))

(fn `UserConstructionScript`)