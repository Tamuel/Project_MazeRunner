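; Maze building piece that places up to four walls around the edges of its Cube surface.
; The construction script reads the Cube's world scale to compute edge offsets, with the second pair of walls rotated 90 degrees.
; MakeWallAtPosition adds a child actor component at unit scale for each enabled Wall1–Wall4 flag.
; The event graph is empty, so all work happens at construction.
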(event `self.ReceiveBeginPlay`)

(event `self.ReceiveActorBeginOverlap`
  (params (OtherActor :type "Actor Object Reference")))

(event `self.ReceiveTick`
  (params (DeltaSeconds :type "Float (single-precision)")))

(fn `MakeWallAtPosition`
  (params (makeOrNot :type Boolean) (position :type "Vector Structure") (rotation :type "Rotator Structure"))
  (if makeOrNot
    (`AddComponent|Child Actor Component_2511` :`RelativeTransform` (`KismetMathLibrary.MakeTransform` position rotation))))

(fn `UserConstructionScript`
  (bind _output_get (set `self.surfaceScale` (`SceneComponent.K2_GetComponentScale` (`self.Cube`))))
  (set `self.surfaceXScale` (.x _output_get))
  (set `self.surfaceYScale` (.y _output_get))
  (`self.MakeWallAtPosition` (`self.wall1`) (`KismetMathLibrary.MakeVector` (* (`self.surfaceXScale`) -5.0) (* (`self.surfaceYScale`) 40.0)))
  (`self.MakeWallAtPosition` (`self.wall2`) (`KismetMathLibrary.MakeVector` (* (`self.surfaceXScale`) -5.0) (* (`self.surfaceYScale`) -50.0)))
  (`self.MakeWallAtPosition` (`self.wall3`) (`KismetMathLibrary.MakeVector` (* (`self.surfaceXScale`) 50.0) (* (`self.surfaceYScale`) -5.0)) (struct :`Yaw` 90.0))
  (`self.MakeWallAtPosition` (`self.wall4`) (`KismetMathLibrary.MakeVector` (* (`self.surfaceXScale`) -40.0) (* (`self.surfaceYScale`) -5.0)) (struct :`Yaw` 90.0)))