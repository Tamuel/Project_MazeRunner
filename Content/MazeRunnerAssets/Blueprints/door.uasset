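; Door actor for the maze runner assets, apparently an unfinished stub for a door that opens when an actor overlaps it.
; Begin and end overlap set the DoorOpen flag and enable ticking, but Tick only checks the flag and moves nothing.
; OpenDoor just returns false.
; MakeWallAtPosition conditionally adds a child actor component at a given location and rotation, and nothing in this Blueprint calls it.
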(event `self.ReceiveBeginPlay`)

(event `self.ReceiveActorBeginOverlap`
  (params (OtherActor :type "Actor Object Reference"))
  (set `self.doorOpen` true)
  (`self.SetActorTickEnabled` true))

(event `self.ReceiveActorEndOverlap`
  (params (OtherActor :type "Actor Object Reference"))
  (set `self.doorOpen` false)
  (`self.SetActorTickEnabled` true))

(event `self.ReceiveTick`
  (params (DeltaSeconds :type "Float (single-precision)"))
  (if (`self.doorOpen`)
    _))

(fn `MakeWallAtPosition`
  (params (makeOrNot :type Boolean) (position :type "Vector Structure") (rotation :type "Rotator Structure"))
  (if makeOrNot
    (`AddComponent|Child Actor Component_2511` :`RelativeTransform` (`KismetMathLibrary.MakeTransform` position rotation))))

(fn `openDoor`
  (returns (end :type Boolean))
  (return false))

(fn `UserConstructionScript`)